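; Lokator is a player-controlled pawn, called Teddy in its comments, that moves and rotates with six degrees of freedom through physics.
; Move and rotate axis inputs apply force and torque to the capsule along the actor's forward, right and up vectors, multiplied by MoveScale and RotationScale.
; Camera axes feed controller yaw, pitch and roll separately, and middle mouse resets control rotation to zero.
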(event EventBeginPlay)

(event EventActorBeginOverlap
  (params (OtherActor :type Actor%20Object%20Reference)))

(event EventTick
  (params (DeltaSeconds :type Float%20%28single-precision%29)))

(event Input|AxisEvents|InputAxisRotateZ
  (params (AxisValue :type Float%20%28single-precision%29))
  ;[1 1 1] Rotate Teddy
  (Class|PrimitiveComponent|AddTorque (Variables|Collision|GetCapsuleComponent) (* (Math|Vector|GetUpVector (Transformation|GetActorRotation)) (* AxisValue (Variables|Default|GetRotationScale))) "None" false))

(event Input|AxisEvents|InputAxisRotateY
  (params (AxisValue :type Float%20%28single-precision%29))
  ;[1 1 1] Rotate Teddy
  (Class|PrimitiveComponent|AddTorque (Variables|Collision|GetCapsuleComponent) (* (Math|Vector|GetRightVector (Transformation|GetActorRotation)) (* AxisValue (Variables|Default|GetRotationScale))) "None" false))

(event Input|AxisEvents|InputAxisRotateX
  (params (AxisValue :type Float%20%28single-precision%29))
  ;[1 1 1] Rotate Teddy
  (Class|PrimitiveComponent|AddTorque (Variables|Collision|GetCapsuleComponent) (* (Math|Vector|GetForwardVector (Transformation|GetActorRotation)) (* AxisValue (Variables|Default|GetRotationScale))) "None" false))

(event Input|AxisEvents|InputAxisMoveX
  (params (AxisValue :type Float%20%28single-precision%29))
  ;[1 1 1] Move Teddy
  (Physics|AddForce (Variables|Collision|GetCapsuleComponent) (* (Math|Vector|GetForwardVector (Transformation|GetActorRotation)) (* AxisValue (Variables|Default|GetMoveScale))) "None" false))

(event Input|AxisEvents|InputAxisCameraRotateZ
  (params (AxisValue :type Float%20%28single-precision%29))
  ;[1 1 1] Rotate camera
  (Pawn|Input|AddControllerYawInput AxisValue))

(event Input|AxisEvents|InputAxisCameraRotateY
  (params (AxisValue :type Float%20%28single-precision%29))
  ;[1 1 1] Rotate camera
  (Pawn|Input|AddControllerPitchInput AxisValue))

(event Input|AxisEvents|InputAxisCameraRotateX
  (params (AxisValue :type Float%20%28single-precision%29))
  ;[1 1 1] Rotate camera
  (Pawn|Input|AddControllerRollInput AxisValue))

(event Input|AxisEvents|InputAxisMoveY
  (params (AxisValue :type Float%20%28single-precision%29))
  ;[1 1 1] Move Teddy
  (Physics|AddForce (Variables|Collision|GetCapsuleComponent) (* (Math|Vector|GetRightVector (Transformation|GetActorRotation)) (* AxisValue (Variables|Default|GetMoveScale))) "None" false))

(event Input|AxisEvents|InputAxisMoveZ
  (params (AxisValue :type Float%20%28single-precision%29))
  ;[1 1 1] Move Teddy
  (Physics|AddForce (Variables|Collision|GetCapsuleComponent) (* (Math|Vector|GetUpVector (Transformation|GetActorRotation)) (* AxisValue (Variables|Default|GetMoveScale))) "None" false))

(event Input|MouseEvents|MiddleMouseButton
  (params (Key :type Key%20Structure :default "AnyKey"))
  ;[1 1 1] Rotate camera
  (:Pressed
    (Pawn|SetControlRotation (Pawn|GetController) (Math|Rotator|MakeRotator 0.0 0.0 0.0))))

(fn ConstructionScript)